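; BP_Door_S is an activable door that swings open and closed around its yaw axis.
; Activation plays a timeline from the start, lerping the door's yaw from closed to DoorOpenRotation, and deactivation reverses it from the end.
; BeginPlay scales the timeline's play rate by OpeningTime and clamps the door's initial yaw.
; The door flags itself busy while moving and clears the flag when the timeline finishes.
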(event `self.ReceiveBeginPlay`
  (bind _door (`self.Door`))
  (bind (_relativerotation_roll _relativerotation_pitch _relativerotation_yaw) (`KismetMathLibrary.BreakRotator` (`SceneComponent.RelativeRotation` _door)))
  (`TimelineComponent.SetPlayRate` (`self.DoorTimeline`) (/ 1.0 (`self.OpeningTime`)))
  (`SceneComponent.K2_SetRelativeRotation` _door (`KismetMathLibrary.MakeRotator` 0.0 0.0 (`KismetMathLibrary.ClampAngle` _relativerotation_yaw 0.0 25.0)) false false))

(event `self.OnActivated`
  (`self.SetBusy` true)
  (bind (_direction _progress) (`Timeline|DoorTimeline` :!via `PlayFromStart` :!label _label)
    (:`Update`
      (`SceneComponent.K2_SetRelativeRotation` (`self.Door`) (`KismetMathLibrary.MakeRotator` 0.0 0.0 (`KismetMathLibrary.Lerp` 0.0 (`self.DoorOpenRotation`) _progress)) false false))
    (:`Finished`
      (`self.SetBusy` false))))

(event `self.OnDeactivated`
  (`self.SetBusy` true)
  (goto _label :!via `ReverseFromEnd`))

(fn `UserConstructionScript`)