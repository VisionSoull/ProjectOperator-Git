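; BP_Lever is a hold-to-interact activator that slides its Lever component and activates its targets when interacted with.
; A timeline, rate-scaled to the required hold duration, moves the lever along Y between normal and active positions.
; Cancelling the hold reverses the timeline and marks the lever busy until its Normal Position event clears that state.
; BeginPlay sets the starting position from the active status.
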(event `self.ReceiveBeginPlay`
  ; Setup base on Active Status
  (`TimelineComponent.SetPlayRate` (`self.LeverTimeline`) (/ 1.0 (`self.GetRequiredHoldDuration`)))
  (`SceneComponent.K2_SetRelativeLocation` (`self.Lever`) (`KismetMathLibrary.MakeVector` 0.0 (`KismetMathLibrary.SelectFloat` (`self.ActivePosition`) (`self.NormalPosition`) (`self.IsActive`))) false false))

(event `self.OnHoldStarted`
  (params (Character :type "Character Object Reference"))
  ; Lever Animation
  (bind (_direction _progress) (`Timeline|LeverTimeline` :!via `PlayFromStart` :!label _label)
    (:`Update`
      (`SceneComponent.K2_SetRelativeLocation` (`self.Lever`) (`KismetMathLibrary.MakeVector` 0.0 (`KismetMathLibrary.Lerp` (`self.NormalPosition`) (`self.ActivePosition`) _progress)) false false))
    (:`OnNormalPosition`
      (`self.SetBusy` false))))

(event `self.OnHoldCancelled`
  (params (Character :type "Character Object Reference"))
  ; Lever Animation
  (`self.SetBusy` true)
  (goto _label :!via `Reverse`))

(event `self.OnInteracted`
  (params (Character :type "Character Object Reference"))
  ; Activate Targets
  (`self.ActivateTargets`))

(fn `UserConstructionScript`)